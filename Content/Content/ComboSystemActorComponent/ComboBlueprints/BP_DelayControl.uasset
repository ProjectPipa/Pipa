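; BP_DelayControl is a short-lived helper actor that times hit input windows for the combo system.
; CheckDelayHit waits the current hit's waiting time, fires CorrectTime, then fires Expired after the hit's remaining time, if any.
; RemainingTime fires Expired after the combo's overall remaining time, when positive.
; Completed timings end with the actor destroying itself after a brief delay.
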(event `CheckDelayHit`
  (bind (_combo_remainingtime _combo_hits) (break `/Game/ComboSystemActorComponent/ComboBlueprints/ST_Combos` (`self.Combo`)))
  (bind (_output_correctcommands _output_nexthittimewaiting _output_nexthitremainingtime) (break `/Game/ComboSystemActorComponent/ComboBlueprints/ST_Hits` (`|GetArrayItem` _combo_hits (`self.Hit`))))
  (`KismetSystemLibrary.Delay` _output_nexthittimewaiting)
  (`self.CorrectTime` (`self.Combo`))
  (if (> _output_nexthitremainingtime 0.0)
    (`KismetSystemLibrary.Delay` _output_nexthitremainingtime)
    (`self.Expired` (`self.Combo`)))
  (`KismetSystemLibrary.Delay` 0.2 :!label _label)
  (`self.K2_DestroyActor`))

(event `RemainingTime`
  (bind _combo_remainingtime (break `/Game/ComboSystemActorComponent/ComboBlueprints/ST_Combos` (`self.Combo`)))
  (if (> _combo_remainingtime 0.0)
    (`KismetSystemLibrary.Delay` _combo_remainingtime)
    (`self.Expired` (`self.Combo`))
    (goto _label)))

(fn `UserConstructionScript`)