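; Base Blueprint for quick time events (QTEs) that passes player input to a QTE component and runs event outcomes.
; Key presses feed the active QTEComponent, and its first configured key starts the QTE when move input is allowed.
; Preset_Event branches on result and preset: Mannequin briefly ragdolls the enemy or player, while Platform failure respawns the player with camera fades.
; PlayCameraAnim plays a given level sequence.
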(event `Key|AnyKey` :consume false :overrideparent false
  (params (Key :type "Key Structure"))
  (bind _qte_component (`self.QTE_Component`))
  ;[1 1 1] Call QTE input on key press
  (:`Pressed`
    (set `self.Gamepad?` (`KismetInputLibrary.Key_IsGamepadKey` Key))
    (`/Engine/EditorBlueprintResources/StandardMacros.IsValid` _qte_component
      (:`Is Valid`
        (`/Game/QTEPack/Blueprints/QTE_Component.Input_Key` _qte_component Key) ; activate input buttons while in QTE
      ))))

(event `Key|AnyKey` :consume false :overrideparent false
  (params (Key :type "Key Structure"))
  (bind _qte_component (`self.QTE_Component`))
  ;[1 1 1] Call QTE input on key press
  (:`Pressed`
    (if (not (`Controller.IsMoveInputIgnored` (`GameplayStatics.GetPlayerController` 0)))
      (`/Engine/EditorBlueprintResources/StandardMacros.IsValid` _qte_component ; if qte component is valid
        (:`Is Valid`
          (bind (_text _texture _key) (`/Game/QTEPack/Blueprints/QTE_Component.Calculate_Button` _qte_component 0)) ; if it is start qte button from key array\n(0) index is the engage qte button
          (if (== _key Key)
            (`/Game/QTEPack/Blueprints/QTE_Component.StartQTE` _qte_component) ; start qte
          ))))))

(event `Preset_Event`
  (params (`Success?` :type Boolean))
  (bind _returnvalue (`GameplayStatics.GetPlayerController` 0))
  (bind _qte_component (`self.QTE_Component`))
  (bind _event_preset (`/Game/QTEPack/Blueprints/QTE_Component.Event_Preset` _qte_component))
  (bind _mesh (`Character.Mesh` (`GameplayStatics.GetPlayerCharacter` 0)))
  ;[0.1553 1 0.095] Event Presets is here, at success and fail you can make what will happen
  ; for example you die when you fail platform QTE
  ; or enemy dies when you success, particles, sounds everything can be stored here
  (`/Engine/EditorBlueprintResources/StandardMacros.IsValid` _qte_component ; check if QTE is still valid to prevent errors
    (:`Is Valid`
      (if `Success?`
        (switch `/Game/QTEPack/Blueprints/Enum_QTEPresets` _event_preset
          (:`NewEnumerator2`
            ;;[1 1 1] choking succes event, temporarily simulate enemy physics
            (bind _asbp_third_person_character (cast `/Game/QTEPack/Starter/Blueprints/BP_ThirdPersonCharacter` (`ActorComponent.GetOwner` (`self.QTE_Component`))))
            (bind _mesh_2 (`Character.Mesh` _asbp_third_person_character))
            (`PrimitiveComponent.SetSimulatePhysics` _mesh_2 true)
            (bind _capsulecomponent (`Character.CapsuleComponent` _asbp_third_person_character))
            (`PrimitiveComponent.SetCollisionResponseToChannel` _capsulecomponent "ECC_Pawn" "ECR_Ignore")
            (`PrimitiveComponent.SetCollisionResponseToChannel` (`TriggerBase.CollisionComponent` (`/Game/QTEPack/Blueprints/QTE_Component.TriggerBox` (`self.GetComponentByClass` _asbp_third_person_character "/Game/QTEPack/Blueprints/QTE_Component.QTE_Component_C"))) "ECC_Pawn" "ECR_Ignore") ; set capsule and QTE trigger box to ignore pawn\n(so we cant activate QTE again while enemy is in ragdoll)
            (`KismetSystemLibrary.Delay` 2.0)
            (`PrimitiveComponent.SetSimulatePhysics` _mesh_2 false)
            (`PrimitiveComponent.SetCollisionResponseToChannel` _capsulecomponent "ECC_Pawn" "ECR_Block") ; set capsule to block pawn
            (`PrimitiveComponent.SetCollisionResponseToChannel` (`TriggerBase.CollisionComponent` (`/Game/QTEPack/Blueprints/QTE_Component.TriggerBox` (`self.GetComponentByClass` _asbp_third_person_character "/Game/QTEPack/Blueprints/QTE_Component.QTE_Component_C"))) "ECC_Pawn" "ECR_Overlap") ; and QTE trigger box to overlap
          ))
        (else
          (switch `/Game/QTEPack/Blueprints/Enum_QTEPresets` _event_preset
            (:`NewEnumerator1`
              ;;[1 1 1] platform fail event, respawn player with camera fade
              (`PlayerCameraManager.StartCameraFade` :`self` (`GameplayStatics.GetPlayerCameraManager` 0) :`ToAlpha` 1.0 :`Duration` 0.5)
              (`self.K2_DestroyActor` (`GameplayStatics.GetPlayerCharacter` 0))
              (bind _outactors (`GameplayStatics.GetAllActorsOfClass` "/Script/Engine.PlayerStart"))
              (bind _returnvalue_2 (`|SpawnActorFromClass` "/Game/QTEPack/Starter/Blueprints/BP_ThirdPersonCharacter.BP_ThirdPersonCharacter_C" (`self.GetTransform` (`|GetArrayItem` _outactors)) "AdjustIfPossibleButAlwaysSpawn" "OverrideRootScale" null null))
              (`Controller.Possess` (`GameplayStatics.GetPlayerController` 0) _returnvalue_2)
              (`PlayerCameraManager.StartCameraFade` :`self` (`GameplayStatics.GetPlayerCameraManager` 0) :`FromAlpha` 1.0 :`ToAlpha` 0.0 :`Duration` 0.5))
            (:`NewEnumerator2`
              ;;[1 1 1] fail while choking, temporarily simulate player's physics and block movement
              (`PrimitiveComponent.SetSimulatePhysics` _mesh true)
              (`Controller.SetIgnoreMoveInput` _returnvalue true)
              (`KismetSystemLibrary.Delay` 1.5)
              (`PrimitiveComponent.SetSimulatePhysics` _mesh false)
              (`Controller.SetIgnoreMoveInput` _returnvalue false))))))))

(fn `PlayCameraAnim`
  (params (LevelSequence :type "LevelSequence Object Reference"))
  (bind (_outactor _returnvalue) (`LevelSequencePlayer.CreateLevelSequencePlayer` LevelSequence))
  (`LevelSequencePlayer.Play` _returnvalue)
  (return))

(fn `UserConstructionScript`)