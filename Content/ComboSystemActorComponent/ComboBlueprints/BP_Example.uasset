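; Example actor for the combo system component, demonstrating cheat-code style combinations entered with number keys.
; Each digit press feeds Hit on the combo component and briefly flashes the digit on three hit texts through a retriggerable delay.
; Completed combos mark their slot and show that code's text as activated, while a wrong hit briefly reveals all three code texts.
; An unconnected snippet shows replacing all combos at runtime.
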(event `Key|One`
  (params (Key :type "Key Structure"))
  (bind _hit_02 (`self.Hit_02`))
  (:`Pressed`
    (`/Game/ComboSystemActorComponent/ComboBlueprints/BPAC_ComboSystem.Hit` (`self.BPAC_ComboSystem`) 1)
    (set `self.Hit` "1")
    (`SceneComponent.SetHiddenInGame` _hit_02 false false :!label _label)
    (`SceneComponent.SetHiddenInGame` (`self.Hit_03`) false false)
    (`SceneComponent.SetHiddenInGame` (`self.Hit_01`) false false)
    (`TextRenderComponent.K2_SetText` _hit_02 (`KismetTextLibrary.Conv_StringToText` (`self.Hit`)))
    (`TextRenderComponent.K2_SetText` (`self.Hit_03`) (`KismetTextLibrary.Conv_StringToText` (`self.Hit`)))
    (`TextRenderComponent.K2_SetText` (`self.Hit_01`) (`KismetTextLibrary.Conv_StringToText` (`self.Hit`)))
    (`KismetSystemLibrary.RetriggerableDelay` 0.35)
    (`SceneComponent.SetHiddenInGame` _hit_02 true false)
    (`SceneComponent.SetHiddenInGame` (`self.Hit_03`) true false)
    (`SceneComponent.SetHiddenInGame` (`self.Hit_01`) true false)))

(event `self.BPAC_ComboSystem.CorrectHits`
  (params (IndexCombo :type Integer) (Hit :type Integer) (LastHit :type Boolean))
  (if LastHit
    (`KismetArrayLibrary.Array_Set` (`self.ComboFinish`) IndexCombo true)
    (`self.UpdateTexts`)
    (`self.SetHiddenTexts`)))

(event `Key|Two`
  (params (Key :type "Key Structure"))
  (:`Pressed`
    (`/Game/ComboSystemActorComponent/ComboBlueprints/BPAC_ComboSystem.Hit` (`self.BPAC_ComboSystem`) 2)
    (set `self.Hit` "2")
    (goto _label)))

(event `Key|Three`
  (params (Key :type "Key Structure"))
  (:`Pressed`
    (`/Game/ComboSystemActorComponent/ComboBlueprints/BPAC_ComboSystem.Hit` (`self.BPAC_ComboSystem`) 3)
    (set `self.Hit` "3")
    (goto _label)))

(event `self.BPAC_ComboSystem.WrongHit`
  (`SceneComponent.SetHiddenInGame` (`self.CheatCode_02`) false false)
  (`SceneComponent.SetHiddenInGame` (`self.CheatCode_03`) false false)
  (`SceneComponent.SetHiddenInGame` (`self.CheatCode_01`) false false)
  (`KismetSystemLibrary.Delay` 0.5)
  (`self.SetHiddenTexts`))

(event `Key|Four`
  (params (Key :type "Key Structure"))
  (:`Pressed`
    (`/Game/ComboSystemActorComponent/ComboBlueprints/BPAC_ComboSystem.Hit` (`self.BPAC_ComboSystem`) 4)
    (set `self.Hit` "4")
    (goto _label)))

(event `self.BPAC_ComboSystem.Expired`
  (params (IndexCombo :type Integer)))

(event `Key|Five`
  (params (Key :type "Key Structure"))
  (:`Pressed`
    (`/Game/ComboSystemActorComponent/ComboBlueprints/BPAC_ComboSystem.Hit` (`self.BPAC_ComboSystem`) 5)
    (set `self.Hit` "5")
    (goto _label)))

(event `Key|Six`
  (params (Key :type "Key Structure"))
  (:`Pressed`
    (`/Game/ComboSystemActorComponent/ComboBlueprints/BPAC_ComboSystem.Hit` (`self.BPAC_ComboSystem`) 6)
    (set `self.Hit` "6")
    (goto _label)))

(event `Key|Seven`
  (params (Key :type "Key Structure"))
  (:`Pressed`
    (`/Game/ComboSystemActorComponent/ComboBlueprints/BPAC_ComboSystem.Hit` (`self.BPAC_ComboSystem`) 7)
    (set `self.Hit` "7")
    (goto _label)))

(event `Key|Eight`
  (params (Key :type "Key Structure"))
  (:`Pressed`
    (`/Game/ComboSystemActorComponent/ComboBlueprints/BPAC_ComboSystem.Hit` (`self.BPAC_ComboSystem`) 8)
    (set `self.Hit` "8")
    (goto _label)))

(event `Key|Nine`
  (params (Key :type "Key Structure"))
  (:`Pressed`
    (`/Game/ComboSystemActorComponent/ComboBlueprints/BPAC_ComboSystem.Hit` (`self.BPAC_ComboSystem`) 9)
    (set `self.Hit` "9")
    (goto _label)))

(event `Key|Zero`
  (params (Key :type "Key Structure"))
  (:`Pressed`
    (`/Game/ComboSystemActorComponent/ComboBlueprints/BPAC_ComboSystem.Hit` (`self.BPAC_ComboSystem`) 0)
    (set `self.Hit` "0")
    (goto _label)))

(fn `SetHiddenTexts`
  (for (_array_element _array_index) (`self.ComboFinish`)
    (switch `int` _array_index
      (:`0`
        (bind _returnvalue (not _array_element))
        (`SceneComponent.SetHiddenInGame` (`self.CheatCode_01`) _returnvalue false))
      (:`1`
        (`SceneComponent.SetHiddenInGame` (`self.CheatCode_02`) _returnvalue false))
      (:`2`
        (`SceneComponent.SetHiddenInGame` (`self.CheatCode_03`) _returnvalue false)))))

(fn `SetTexts`
  (params (Text :type "TextRenderComponent Object Reference") (bCorrect :type Boolean))
  (`TextRenderComponent.K2_SetText` Text (`KismetTextLibrary.Conv_StringToText` (`KismetMathLibrary.SelectString` "CHEAT CODE ACTIVATE" "WRONG COMBINATION" bCorrect))))

(fn `UpdateTexts`
  (for (_array_element _array_index) (`self.ComboFinish`)
    (switch `int` _array_index
      (:`0`
        (`self.SetTexts` (`self.CheatCode_01`) _array_element))
      (:`1`
        (`self.SetTexts` (`self.CheatCode_02`) _array_element))
      (:`2`
        (`self.SetTexts` (`self.CheatCode_03`) _array_element)))))

(fn `UserConstructionScript`)